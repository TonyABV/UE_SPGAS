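; Event-activated gameplay ability that fires a single hitscan shot from the equipped weapon.
; Only when HasAuthority is false, it plays the weapon's attack montage and waits once for the Event.Combat.Shoot gameplay event.
; That event line-traces from the muzzle along control rotation and applies the weapon's damage effect to the hit actor's ability system component.
; The ability ends when the montage finishes or the shot finds no valid target.
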(event Custom|Shoot
  (bind _returnvalue (Class|GAInventoryAbility|GetEquippedWeaponItemActor))
  (bind _returnvalue_2 (Class|WeaponItemActor|GetMuzzleLocation _returnvalue))
  (bind (_outhit _returnvalue_3) (Collision|LineTraceByChannel _returnvalue_2 (+ _returnvalue_2 (* (Pawn|GetControlRotation (.playercontroller (Ability|GetActorInfo)) :!class /Script/Engine.Controller) (Variables|Default|GetShootingDistance))) "TraceTypeQuery1" false 0 "ForDuration"))
  (if _returnvalue_3
    (Utilities|IsValid (Ability|GetAbilitySystemComponent (.HitActor (Collision|BreakHitResult _outhit)))
      (:Is%20Valid
        (GameplayEffects|ApplyGameplayEffectToSelf :self (Ability|GetAbilitySystemComponent (.HitActor (Collision|BreakHitResult _outhit))) :GameplayEffectClass (Variables|/Script/StudyProject.WeaponStaticData|GetDamageEffect (Class|GAInventoryAbility|GetEquippedWeaponStaticData))))
      (:Is%20Not%20Valid
        (Ability|EndAbility :!label _label)))
    (else
      (goto _label))))

(event Ability|EventActivateAbilityFromEvent
  (params (EventData :type Gameplay%20Event%20Data%20Structure%20%28by%20ref%29))
  (Ability|HasAuthority
    (:False
      (|PlayMontageandWaitProxy "None" (Variables|/Script/StudyProject.WeaponStaticData|GetAttackMontage (Class|GAInventoryAbility|GetEquippedWeaponStaticData)) 1.0 "None" true 1.0 0.0
        (:then
          (Ability|Tasks|WaitGameplayEvent "(TagName=\"Event.Combat.Shoot\")" 0 true
            (:EventReceived
              (CallFunction|Shoot))))
        (:OnCompleted
          (Ability|EndAbility :!label _label))
        (:OnBlendOut
          (goto _label))
        (:OnInterrupted
          (goto _label))
        (:OnCancelled
          (goto _label))))))