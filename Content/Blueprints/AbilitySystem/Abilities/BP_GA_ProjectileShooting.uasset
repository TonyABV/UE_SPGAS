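; Gameplay ability that fires a rocket projectile from the character's equipped weapon.
; On activation it traces from the weapon toward the focus point and passes the hit result to the weapon's effects.
; It then launches a projectile using the rocket static data along the trace direction, spawned at an offset from the muzzle with the character as owner and instigator, and immediately ends the ability.
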(event Ability|EventActivateAbility
  (bind _returnvalue (Class|SPGameplayAbility|GetSPCharacter))
  (bind _shootingdistance (Variables|Default|GetShootingDistance))
  (bind _outhitresult (Class|GAInventoryCombatAbility|GetWeapontoFocusTraceResult _shootingdistance "TraceTypeQuery3"))
  (bind _returnvalue_2 (- (.traceend _outhitresult) (.tracestart _outhitresult)))
  (bind _returnvalue_3 (Math|Vector|Normalize _returnvalue_2))
  (Class|WeaponItemActor|PlayWeaponEffects (Class|GAInventoryAbility|GetEquippedWeaponItemActor) (Collision|MakeHitResult (.bblockinghit _outhitresult) (.binitialoverlap _outhitresult) (.time _outhitresult) (.distance _outhitresult) (.location _outhitresult) (.impactpoint _outhitresult) (.normal _outhitresult) (.impactnormal _outhitresult) 0 0 0 "None" "None" 0 0 0 (.tracestart _outhitresult) (.traceend _outhitresult)))
  (Class|SPStatics|LaunchProjectile "/Game/Blueprints/Inventory/Items/BP_RocketStaticData.BP_RocketStaticData_C" (Math|Transform|MakeTransform (+ (Class|WeaponItemActor|GetMuzzleLocation (Class|GAInventoryAbility|GetEquippedWeaponItemActor)) (* _returnvalue_3 (Variables|Default|GetSpawnOffset))) (Math|Conversions|RotationFromXVector _returnvalue_3)) _returnvalue _returnvalue)
  (Ability|EndAbility))

(event Ability|EventOnEndAbility
  (params (bWasCancelled :type Boolean)))