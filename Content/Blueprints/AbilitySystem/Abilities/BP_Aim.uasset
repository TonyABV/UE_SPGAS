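; BP_Aim is a gameplay ability that applies an aiming camera effect to the player while aiming is active.
; On activation it adds BP_AimCameraModifier to the player camera manager, stores the handle, and waits for the Event.Combat.Aim.Ended gameplay event to end itself.
; It ends immediately if no valid controller or camera manager exists, and removes the stored modifier whenever the ability ends.
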(event Ability|EventActivateAbility
  (bind _returnvalue (Ability|GetActorInfo))
  (Utilities|IsValid (.playercontroller _returnvalue)
    (:Is%20Valid
      (bind _playercameramanager (Variables|/Script/Engine.PlayerController|GetPlayerCameraManager (.playercontroller _returnvalue))
        (:then
          (bind _returnvalue_2 (Game|Player|AddNewCameraModifier _playercameramanager "/Game/Blueprints/CameraModifire/BP_AimCameraModifier.BP_AimCameraModifier_C"))
          (Variables|Default|SetAimCameraModifierHandle _returnvalue_2)
          (Ability|Tasks|WaitGameplayEvent "(TagName=\"Event.Combat.Aim.Ended\")" 0
            (:EventReceived
              _)))
        (:else
          _)))
    (:Is%20Not%20Valid
      _))
  (Ability|EndAbility))

(event Ability|EventOnEndAbility
  (params (bWasCancelled :type Boolean))
  (bind _returnvalue (Ability|GetActorInfo))
  (Utilities|IsValid (.playercontroller _returnvalue)
    (:Is%20Valid
      (bind _playercameramanager (Variables|/Script/Engine.PlayerController|GetPlayerCameraManager (.playercontroller _returnvalue))
        (:then
          (Game|Player|RemoveCameraModifier _playercameramanager (Variables|Default|GetAimCameraModifierHandle)))
        (:else)))))